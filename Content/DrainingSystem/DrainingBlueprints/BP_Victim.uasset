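; BP_Victim is a blood-draining target that loses Health as the player collides with it.
; Each capsule hit from the player pawn decrements Health, and while Health stays above zero a colliding BP_ThirdPersonCharacter gains BloodLevel.
; Every tick it writes Health to the WB_Victim_BloodLevel progress bar and rotates that widget component to face the player camera.
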(event `self.CapsuleComponent.OnComponentHit`
  (params (HitComponent :type "PrimitiveComponent Object Reference") (OtherActor :type "Actor Object Reference") (OtherComp :type "PrimitiveComponent Object Reference") (NormalImpulse :type "Vector Structure") (Hit :type "HitResult Structure (by ref)"))
  ; Decrease Victim Blood Levels
  (`|ExecutionSequence`
    (:`then_0`
      (if (== (`GameplayStatics.GetPlayerPawn` 0) OtherActor)
        (bind _result (`/Engine/EditorBlueprintResources/StandardMacros.DecrementFloat` (`self.Health`))
          (:`  `
            (set `self.Health` _result)))))
    (:`then_1`
      ; Increase Player Blood Level
      (if (> (`self.Health`) 0.0)
        (bind _asbp_third_person_character (cast `/Game/ThirdPerson/Blueprints/BP_ThirdPersonCharacter` OtherActor))
        (bind _result_2 (`/Engine/EditorBlueprintResources/StandardMacros.IncrementFloat` (`/Game/ThirdPerson/Blueprints/BP_ThirdPersonCharacter.BloodLevel` _asbp_third_person_character))
          (:`  `
            (set `/Game/ThirdPerson/Blueprints/BP_ThirdPersonCharacter.BloodLevel` _result_2 _asbp_third_person_character)))))))

(event `self.ReceiveTick`
  (params (DeltaSeconds :type "Float (single-precision)"))
  (bind _widget_bloodlevel (`self.Widget_BloodLevel`))
  ; Health/Blood Bar
  (bind _aswb_victim_blood_level (cast `/Game/DrainingSystem/DrainingBlueprints/WB_Victim_BloodLevel` (`WidgetComponent.GetWidget` (`self.Widget_BloodLevel`))))
  (`ProgressBar.SetPercent` (`/Game/DrainingSystem/DrainingBlueprints/WB_Victim_BloodLevel.HealthBar` _aswb_victim_blood_level) (/ (`self.Health`) 100.0))
  (`SceneComponent.K2_SetWorldRotation` _widget_bloodlevel (`KismetMathLibrary.FindLookAtRotation` (`SceneComponent.K2_GetComponentLocation` _widget_bloodlevel) (`SceneComponent.K2_GetComponentLocation` (`PlayerCameraManager.TransformComponent` (`GameplayStatics.GetPlayerCameraManager` 0)))) false false))

(fn `UserConstructionScript`)