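; BP_Door is an interactable door that toggles between open and closed on Interact, playing a sound at its location each time.
; A timeline drives the Door component's yaw, playing forward to open and in reverse to close.
; Interaction query functions supply the prompt for the current state, a marker component's location, the interaction type, hold duration and tap count.
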(event `OpenDoor`
  ;[0 0.1346 0.15 0.5 20] Interact
  (set `self.IsOpen` true)
  (`GameplayStatics.PlaySoundAtLocation` "/Engine/VREditor/Sounds/UI/Enter_Simulate.Enter_Simulate" (`self.K2_GetActorLocation`) (struct) 1.0 1.0 0.0 null null null null)
  (bind (_direction _zrotation) (`Timeline|OpenDoorTimeline` :!label _label)
    (:`Update`
      (`SceneComponent.K2_SetRelativeRotation` (`self.Door`) (`KismetMathLibrary.MakeRotator` 0.0 0.0 _zrotation) false false))))

(event `CloseDoor`
  ;[0 0.1346 0.15 0.5 20] Interact
  (set `self.IsOpen` false)
  (`GameplayStatics.PlaySoundAtLocation` "/Engine/VREditor/Sounds/UI/Leave_Simulate.Leave_Simulate" (`self.K2_GetActorLocation`) (struct) 1.0 1.0 0.0 null null null null)
  (goto _label :!via `Reverse`))

(event `/Game/InteractionSystem/Blueprints/BPI_Interactable.Interact`
  (params (Interactor :type "Actor Object Reference"))
  ;[0 0.1346 0.15 0.5 20] Interact
  (if (`self.IsOpen`)
    (`self.CloseDoor`)
    (else
      (`self.OpenDoor`))))

(fn `GetHoldDuration`
  (returns (Duration :type "Float (double-precision)"))
  ;[0 0.07582 0.15 0.5 14] Interact
  (return 0.0))

(fn `GetInteractionLocation`
  (returns (Location :type "Vector Structure"))
  (return (`SceneComponent.K2_GetComponentLocation` (`self.InteractionLocation`))))

(fn `GetInteractionPrompt`
  (returns (Value :type Text))
  ;[0.003716 0.1169 0.15 0.5 14] Interact
  (return (select `bool` (`self.IsOpen`) :`false` "to open the door" :`true` "to close the door" :!type "Text")))

(fn `GetInteractionType`
  (returns (Type :type "/Game/InteractionSystem/Blueprints/E_InteractionType Enum"))
  ;[0.008268 0.1168 0.15 0.5 14] Interact
  (return "NewEnumerator0"))

(fn `GetTapCount`
  (returns (Value :type Integer))
  (return 4))

(fn `UserConstructionScript`)