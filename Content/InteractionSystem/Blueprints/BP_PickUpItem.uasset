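; BP_PickUpItem is an interactable pickup actor for the interaction system that stands in for collecting an item.
; Interact prints an "added to inventory" message naming the item and interactor, plays a sound at the world origin, then destroys the actor; no inventory is updated.
; Its interaction getters return the HoldDuration variable, the enum's NewEnumerator0 type, and empty or zero prompt, location and tap count.
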(event `/Game/InteractionSystem/Blueprints/BPI_Interactable.Interact`
  (params (Interactor :type "Actor Object Reference"))
  ;[0 0.15 0.146 0.5 20] Interact System
  (`KismetSystemLibrary.PrintString` (`KismetTextLibrary.Conv_TextToString` (`|FormatText` "Added {ItemName} to the inventory of {ActorName}" (`KismetSystemLibrary.GetDisplayName` self) (`KismetSystemLibrary.GetDisplayName` Interactor))))
  (`GameplayStatics.PlaySoundAtLocation` "/Engine/VREditor/Sounds/UI/Dockable_Window_Close.Dockable_Window_Close" (0.0 0.0 0.0) (struct) 1.0 1.0 0.0 null null null null)
  (`self.K2_DestroyActor`))

(fn `GetHoldDuration`
  (returns (Duration :type "Float (double-precision)"))
  (return (`self.Hold Duration`)))

(fn `GetInteractionLocation`
  (returns (Location :type "Vector Structure"))
  (return (0.0 0.0 0.0)))

(fn `GetInteractionPrompt`
  (returns (Value :type Text))
  (return ""))

(fn `GetInteractionType`
  (returns (Type :type "/Game/InteractionSystem/Blueprints/E_InteractionType Enum"))
  ;[0.00062 0.1107 0.15 0.5 14] Interact
  (return "NewEnumerator0"))

(fn `GetTapCount`
  (returns (Value :type Integer))
  (return 0))

(fn `UserConstructionScript`)