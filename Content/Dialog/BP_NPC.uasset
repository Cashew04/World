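; BP_NPC is a talkable NPC that steps through its Dialogue lines each time its Talk interface event fires.
; Each call increments TalkIndex: with no widget it creates and shows WB_Dialogue without setting text; otherwise it sets TalkText to the indexed line and plays a sound at world origin.
; When the index passes the last line, it removes the widget and resets the index and UI reference.
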(event `/Game/Dialog/BPI_Dialog.Talk`
  ; Dialogue from interfaces
  (`/Engine/EditorBlueprintResources/StandardMacros.IncrementInt` (`self.TalkIndex`)
    (:`  `
      (if (< (`self.TalkIndex`) (`KismetArrayLibrary.Array_Length` (`self.Dialogue`)))
        (`self.UI`
          (:`then`
            (`TextBlock.SetText` (`/Game/Dialog/WB_Dialogue.TalkText` (`self.UI`)) (`KismetTextLibrary.Conv_StringToText` (`|GetArrayItem` (`self.Dialogue`) (`self.TalkIndex`))))
            (`GameplayStatics.PlaySoundAtLocation` "/Engine/VREditor/Sounds/UI/Dockable_Window_Open.Dockable_Window_Open" (0.0 0.0 0.0) (struct) 1.0 1.0 0.0 null null null null))
          (:`else`
            (bind _returnvalue (`|CreateWidget` "/Game/Dialog/WB_Dialogue.WB_Dialogue_C" (`GameplayStatics.GetPlayerController` 0)))
            (bind _output_get (set `self.UI` _returnvalue))
            (`UserWidget.AddToViewport` _output_get 0)))
        (else
          (`Widget.RemoveFromParent` (`self.UI`))
          (set `self.TalkIndex` 0)
          (set `self.UI` null))))))

(fn `UserConstructionScript`)